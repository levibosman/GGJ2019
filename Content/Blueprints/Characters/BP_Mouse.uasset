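; BP_Mouse is a mouse character that can pick up, carry and throw another mouse.
; Interacting with an available mouse registers it as the interactor's CarriedMouse, with CanInteract gated on the interactor controller's CharacterType.
; Tick snaps the carried mouse to MouseLiftLocation.
; The Throwing input launches it toward HoldLocation's direction with a throw montage, or calls DropObject when no mouse is carried.
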(event `self.ReceiveTick`
  (params (DeltaSeconds :type "Float (single-precision)"))
  (`parent.ReceiveTick` DeltaSeconds)
  (`self.HandlePickingUp`))

(event `/Game/Blueprints/Interfaces/BPI_Interacbility.OnInteract`
  (params (Interactee :type "/Game/Blueprints/Characters/BP_Character Object Reference"))
  (if (`self.CanBePickedUp`)
    (`self.PickedUp` Interactee)))

(event `InputAction|Throwing`
  (params (Key :type "Key Structure"))
  (:`Pressed`
    (`/Engine/EditorBlueprintResources/StandardMacros.IsValid` (`self.CarriedMouse`)
      (:`Is Valid`
        (`self.YEETmouse`))
      (:`Is Not Valid`
        (`self.DropObject` true)))))

(fn `CanInteract`
  (params (Interactee :type "/Game/Blueprints/Characters/BP_Character Object Reference"))
  (returns (`CanInteract?` :type Boolean))
  (bind _asbp_player_controller (cast `/Game/Blueprints/Controllers/BP_PlayerController` (`self.GetController` Interactee)))
  (return (`|EnumEquality` (`/Game/Blueprints/Controllers/BP_PlayerController.CharacterType` _asbp_player_controller) "NewEnumerator1")))

(fn `HandlePickingUp`
  (bind _carriedmouse (`self.CarriedMouse`))
  (if (`self.PickingUp`)
    (`/Engine/EditorBlueprintResources/StandardMacros.IsValid` _carriedmouse
      (:`Is Valid`
        (`self.K2_SetActorLocation` _carriedmouse (`SceneComponent.K2_GetComponentLocation` (`self.MouseLiftLocation`)) false false)))))

(fn `PickedUp`
  (params (Interactee :type "/Game/Blueprints/Characters/BP_Character Object Reference"))
  (bind _asbp_mouse (cast `/Game/Blueprints/Characters/BP_Mouse` Interactee))
  (if (not (`/Game/Blueprints/Characters/BP_Mouse.PickingUp` _asbp_mouse))
    (set `/Game/Blueprints/Characters/BP_Mouse.CarriedMouse` self _asbp_mouse)
    (set `self.CanBePickedUp` false)
    (set `/Game/Blueprints/Characters/BP_Mouse.PickingUp` true _asbp_mouse)))

(fn `UserConstructionScript`
  (`parent.UserConstructionScript`))

(fn `YEETmouse`
  (set `self.PickingUp` false)
  (`self.K2_SetActorLocation` (`self.CarriedMouse`) (`SceneComponent.K2_GetComponentLocation` (`self.MouseLiftLocation`)) false false)
  (`self.LaunchCharacter` (`self.CarriedMouse`) (* (`KismetMathLibrary.GetForwardVector` (`KismetMathLibrary.FindLookAtRotation` (`self.K2_GetActorLocation`) (`SceneComponent.K2_GetComponentLocation` (`self.HoldLocation`)))) (`self.MouseThrowForce`)) true true)
  (set `/Game/Blueprints/Characters/BP_Mouse.CanBePickedUp` true (`self.CarriedMouse`))
  (set `self.CarriedMouse` null)
  (`self.PlayAnimMontage` "/Game/Art/Animations/Mouse/Anim_Throw.Anim_Throw"))